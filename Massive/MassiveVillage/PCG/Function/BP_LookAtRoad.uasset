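; Custom PCG Blueprint node "Look at road" that turns points in the Massive Village generation to face roads.
; It caches locations from the "Road Location Point" input, then loops over the main input's points, searching those locations by 2D distance.
; Each point's yaw aims at the chosen road location plus an offset, keeping pitch and roll, with density set to one.
; An optional debug sphere marks the target; an older sphere-trace search is left unused.
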(fn ExecutewithContext
  (params (InContext :type PCG%20Context%20Structure%20%28by%20ref%29) (Input :type PCG%20Data%20Collection%20Structure%20%28by%20ref%29))
  (CallFunction|GetAllRoadPointsLocation Input)
  (bind _returnvalue (Class|PCGDataFunctionLibrary|GetInputs Input))
  (if (> (Utilities|Array|Length _returnvalue) 0)
    (bind _aspcgspatial_data (Utilities|Casting|CastToPCGSpatialData (.Data (Utilities|Struct|BreakPCGTaggedData (Utilities|Array|Get(acopy) _returnvalue)))))
    (bind _outdata (PCG|FlowControl|PointLoop InContext (SpatialData|ToPointDatawithContext _aspcgspatial_data InContext) 0))
    (Variables|/Script/PCG.PCGSpatialData|SetTargetActor _outdata (Variables|/Script/PCG.PCGSpatialData|GetTargetActor _aspcgspatial_data))
    (return (Utilities|Struct|MakePCGDataCollection (Utilities|Array|MakeArray (Utilities|Struct|MakePCGTaggedData _outdata 0 "None"))))
    (else
      (return ""))))

(fn PointLoopBody
  (params (InContext :type PCG%20Context%20Structure%20%28by%20ref%29) (InData :type PCG%20Point%20Data%20Object%20Reference) (InPoint :type PCG%20Point%20Structure%20%28by%20ref%29) (OutMetadata :type PCG%20Metadata%20Object%20Reference) (Iteration :type Integer64))
  (LocalVariables|SetPoint%20Transform (Utilities|Struct|BreakPCGPoint InPoint))
  (if (> (Utilities|Array|Length (Variables|Default|GetAllRoadPointsLocation)) 0)
    (for _array_element (Variables|Default|GetAllRoadPointsLocation)
      (if (< (Math|Vector|Distance2D(Vector) (.location (LocalVariables|GetPoint%20Transform)) _array_element) (LocalVariables|GetClosest%20Point))
        (LocalVariables|SetClosest%20Point (Math|Vector|Distance2D(Vector) (.location (LocalVariables|GetPoint%20Transform)) _array_element))
        (LocalVariables|SetLookAtPosition _array_element)))
    (bind _structout (Utilities|Struct|SetmembersinPCGPoint InPoint (Math|Transform|MakeTransform (.location (LocalVariables|GetPoint%20Transform)) (Math|Rotator|MakeRotator (.roll (.rotation (LocalVariables|GetPoint%20Transform))) (.pitch (.rotation (LocalVariables|GetPoint%20Transform))) (+ (.yaw (Math|Rotator|FindLookatRotation (.location (LocalVariables|GetPoint%20Transform)) (LocalVariables|GetLookAtPosition))) (Variables|Default|GetRotation%20Offset))) (.scale (LocalVariables|GetPoint%20Transform)))))
    (if (Variables|Default|GetDebug%20Look%20At%20Position)
      (Rendering|Debug|DrawDebugSphere (LocalVariables|GetLookAtPosition) 2e+02 12 "(R=1.000000,G=0.000000,B=0.029930,A=1.000000)" 5.0 1e+01))
    (return _structout true)
    (else
      (Development|PrintString "could not find roads"))))

(fn NodeTitleOverride
  (return "Look at road"))

(fn GetAllRoadPointsLocation
  (params (InCollection :type PCG%20Data%20Collection%20Structure%20%28by%20ref%29))
  (Utilities|Array|Clear (Variables|Default|GetAllRoadPointsLocation))
  (bind _returnvalue (Data|GetTypedInputsbyPinLabel InCollection "Road Location Point" 0))
  (bind _aspcgpoint_data (Utilities|Casting|CastToPCGPointData (Utilities|Array|Get(acopy) _returnvalue)))
  (for _array_element (SpatialData|GetPoints _aspcgpoint_data)
    (Utilities|Array|Add (Variables|Default|GetAllRoadPointsLocation) (.location (Utilities|Struct|BreakPCGPoint _array_element))))
  (return))