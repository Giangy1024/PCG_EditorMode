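; BP_Road2_0 is a spline-based road actor that refreshes its helper components in the construction script through UpdateRoad.
; It raises End above spline point 1 and Billboard above the midpoint of points 0 and 1.
; When a SplineMeshComponent exists, it sets PCGSpline to None, then attempts custom primitive data writes on that empty reference.
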(fn ConstructionScript
  (CallFunction|UpdateRoad))

(fn UpdateRoad
  (bind _spline (Variables|Default|GetSpline))
  (bind _spline_2 (Variables|Default|GetSpline))
  (bind _spline_3 (Variables|Default|GetSpline))
  (bind _returnvalue (Spline|GetTransformatSplinePoint _spline 0 "World" false))
  (bind _returnvalue_2 (Spline|GetTransformatSplinePoint _spline_3 1 "World" false))
  (bind _returnvalue_3 (Spline|GetTransformatSplinePoint _spline_2 1 "World" false))
  (bind _returnvalue_4 (+ (.location _returnvalue_2) (.location _returnvalue)))
  (bind _returnvalue_5 (/ _returnvalue_4 "2.000000,2.000000,2.000000"))
  (Transformation|SetWorldLocation (Variables|Default|GetEnd) (Math|Vector|MakeVector (.x (.location _returnvalue_3)) (.y (.location _returnvalue_3)) (+ (.z (.location _returnvalue_3)) 2e+03)) false false)
  (Transformation|SetWorldLocation (Variables|Default|GetBillboard) (Math|Vector|MakeVector (.x _returnvalue_5) (.y _returnvalue_5) (+ (.z _returnvalue_5) 5e+03)) false false)
  (Utilities|IsValid (Actor|GetComponentbyClass "/Script/Engine.SplineMeshComponent")
    (:Is%20Valid
      (bind _output_get (LocalVariables|SetPCG%20Spline 0))
      (Rendering|Material|SetCustomPrimitiveDataFloat _output_get 0 0.0)
      (Rendering|Material|SetCustomPrimitiveDataFloat _output_get (Spline|GetNumberOfSplinePoints (LocalVariables|GetPCG%20Spline)) 1.0))))