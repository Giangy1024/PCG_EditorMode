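; Farm generator actor for Massive Village that runs a PCG graph from its construction script.
; Generate derives fence and dirt spacing from each list's first mesh bounds, then fits the box to the actor's bounds before generating.
; Separate functions push mesh lists to graph parameters, clean up or destroy generated content, and toggle editor auto-regeneration with a billboard indicator.
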(fn ConstructionScript
  (CallFunction|Generate))

(fn Destroy
  (for _array_element (Actor|GetAttachedActors true false)
    (Utilities|Array|AddUnique (LocalVariables|GetAllActors) _array_element))
  (for _array_element_2 (LocalVariables|GetAllActors)
    (Actor|DestroyActor _array_element_2))
  (Actor|DestroyActor))

(fn Generate
  (bind (_origin _boxextent) (Collision|GetActorBounds false true))
  (bind _box (Variables|Default|GetBox))
  (Class|PCGComponent|SetGraph (Variables|Default|GetPCG) (Variables|Global|GetPCG%20Graph))
  (bind _fence (Variables|Building|GetFence)
    (:then
      (CallFunction|GetFarmFenceList _fence)
      (bind _dirt (Variables|Crop|GetDirt)
        (:then
          (CallFunction|GetFarmDirtList _dirt))
        (:else
          _))
      (LocalVariables|SetOrigin _origin)
      (LocalVariables|SetExtend _boxextent)
      (Transformation|SetWorldLocation _box (LocalVariables|GetOrigin) false true)
      (Components|Box|SetBoxExtent _box (LocalVariables|GetExtend) true)
      (PCG|Generate (Variables|Default|GetPCG) false)
      (Transformation|SetWorldLocation (Variables|Default|GetBillboard) (Math|Vector|MakeVector (.x (LocalVariables|GetOrigin)) (.y (LocalVariables|GetOrigin)) (+ (.z (LocalVariables|GetOrigin)) 1e+03)) false false))
    (:else)))

(fn GetMassiveVillageData
  (return))

(fn UpdateMeshLists
  (Audio|Parameter|SetObjectParameter (Variables|/Script/PCG.PCGComponent|GetGraphInstance (Variables|Default|GetPCG)) "BuildingList" (Variables|Building|GetBuilding))
  (Audio|Parameter|SetObjectParameter (Variables|/Script/PCG.PCGComponent|GetGraphInstance (Variables|Default|GetPCG)) "CropsList" (Variables|Crop|GetCrops))
  (Audio|Parameter|SetObjectParameter (Variables|/Script/PCG.PCGComponent|GetGraphInstance (Variables|Default|GetPCG)) "FenceList" (Variables|Building|GetFence))
  (Audio|Parameter|SetObjectParameter (Variables|/Script/PCG.PCGComponent|GetGraphInstance (Variables|Default|GetPCG)) "ScarecrowList" (Variables|Crop|GetScarecrow))
  (Audio|Parameter|SetObjectParameter (Variables|/Script/PCG.PCGComponent|GetGraphInstance (Variables|Default|GetPCG)) "SmallFenceList" 0)
  (Audio|Parameter|SetObjectParameter (Variables|/Script/PCG.PCGComponent|GetGraphInstance (Variables|Default|GetPCG)) "RoadList" (Variables|Road|GetRoad))
  (Audio|Parameter|SetObjectParameter (Variables|/Script/PCG.PCGComponent|GetGraphInstance (Variables|Default|GetPCG)) "DirtList" (Variables|Crop|GetDirt))
  (return))

(fn GetFarmFenceList
  (params (Target :type PDA%20Village%20Object%20Object%20Reference))
  (bind _structout (Utilities|Struct|SetmembersinST_Object (Utilities|Array|Get(acopy) (Variables|/Game/Massive/MassiveVillage/Data/Structure/PDA_VillageObject.PDA_VillageObject_C|GetMeshes Target))))
  (Variables|Data|SetVillageFenceLength (Math|Float|Clamp(Float) (* (.x (.boxextent (StaticMesh|GetBounds (.mesh _structout)))) 2.0) 25.0 1e+03))
  (return))

(fn GetSmallFenceList
  (params (Target :type PDA%20Village%20Object%20Object%20Reference))
  (bind _structout (Utilities|Struct|SetmembersinST_Object (Utilities|Array|Get(acopy) (Variables|/Game/Massive/MassiveVillage/Data/Structure/PDA_VillageObject.PDA_VillageObject_C|GetMeshes Target))))
  (Variables|Data|SetHouseFenceLength (Math|Float|Clamp(Float) (* (.x (.boxextent (StaticMesh|GetBounds (.mesh _structout)))) 2.0) 25.0 1e+03))
  (return))

(fn GetFarmDirtList
  (params (Target :type PDA%20Village%20Object%20Object%20Reference))
  (bind _structout (Utilities|Struct|SetmembersinST_Object (Utilities|Array|Get(acopy) (Variables|/Game/Massive/MassiveVillage/Data/Structure/PDA_VillageObject.PDA_VillageObject_C|GetMeshes Target))))
  (Variables|Data|SetDirtMeshSize (Math|Float|Clamp(Float) (* (.x (.boxextent (StaticMesh|GetBounds (.mesh _structout)))) 2.0) 25.0 1e+03))
  (return))

(fn Clear
  (Class|PCGComponent|Cleanup (Variables|Default|GetPCG) true false))

(fn ToggleAutoPCGUpdate
  (if (Variables|Data|GetUpdateLandscape?)
    ;[0.02522 0.249 0.07835] Auto Update PCG
    (Variables|Data|SetUpdateLandscape? false)
    (Variables|/Script/PCG.PCGComponent|SetbRegenerateInEditor (Variables|Default|GetPCG) true)
    (Rendering|SetVisibility (Variables|Default|GetBillboardUpdate) true false)
    (PCG|Generate (Variables|Default|GetPCG) true)
    (else
      ;[1 0.2691 0.2433] Stop Auto Update PCG
      (Variables|Data|SetUpdateLandscape? true)
      (Variables|/Script/PCG.PCGComponent|SetbRegenerateInEditor (Variables|Default|GetPCG) false)
      (Rendering|SetVisibility (Variables|Default|GetBillboardUpdate) false false)
      (PCG|Generate (Variables|Default|GetPCG) true))))