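; BP_RemoveSpline is a spline actor that marks where vegetation, buildings or both are to be excluded in MassiveVillage, apparently for other generators to read.
; On construction it rebuilds its NoVegetation and NoBuilding actor tags from two flags and picks a matching billboard sprite.
; It also averages the local spline point positions to float that icon above the approximate center of the spline.
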(fn ConstructionScript
  (CallFunction|ForceUpdate)
  (CallFunction|GetCenterPosition))

(fn ForceUpdate
  (Utilities|Array|Clear (Variables|Actor|GetTags))
  (Utilities|FlowControl|Sequence
    (:then_0
      (if (Variables|Default|GetRemove%20Vegetation)
        (Utilities|Array|AddUnique (Variables|Actor|GetTags) "NoVegetation")
        (if (Variables|Default|GetRemove%20Building)
          (Rendering|Components|Sprite|SetSprite (Variables|Default|GetBillboardIcon) "/Game/Massive/MassiveVillage/Texture/UI/BuildingAndTree.BuildingAndTree" :!label _label)
          (else
            (Rendering|Components|Sprite|SetSprite (Variables|Default|GetBillboardIcon) "/Game/Massive/MassiveVillage/Texture/UI/Tree.Tree")))))
    (:then_1
      (if (Variables|Default|GetRemove%20Building)
        (Utilities|Array|AddUnique (Variables|Actor|GetTags) "NoBuilding")
        (if (Variables|Default|GetRemove%20Vegetation)
          (goto _label)
          (else
            (Rendering|Components|Sprite|SetSprite (Variables|Default|GetBillboardIcon) "/Game/Massive/MassiveVillage/Texture/UI/Resident.Resident")))))))

(fn GetCenterPosition
  (bind _spline (Variables|Default|GetSpline))
  (bind _returnvalue (Spline|GetNumberOfSplinePoints _spline))
  (LocalVariables|SetPositionSum "0, 0, 0")
  (Utilities|Array|Clear (LocalVariables|GetPosition))
  (LocalVariables|SetNumber%20of%20Points _returnvalue)
  (for _index (range 1 _returnvalue)
    (Utilities|Array|AddUnique (LocalVariables|GetPosition) (.position (Spline|GetSplinePointAt (Variables|Default|GetSpline) _index "Local"))))
  (for _array_element (LocalVariables|GetPosition)
    (LocalVariables|SetPositionSum (+ (LocalVariables|GetPositionSum) _array_element)))
  (Transformation|SetRelativeLocation (Variables|Default|GetBillboardIcon) (+ (/ (LocalVariables|GetPositionSum) (LocalVariables|GetNumber%20of%20Points)) "0.000000,0.000000,500.000000") false false))