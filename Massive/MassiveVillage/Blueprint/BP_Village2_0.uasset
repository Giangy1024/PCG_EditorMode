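; BP_Village2_0 is a spline-based village generator actor driven by a PCG graph.
; Construction assigns the graph and, given a valid Fence, derives fence length from mesh bounds and fits a cube and billboard to the actor bounds.
; Helper functions nudge the spline to force regeneration, clear PCG output and toggle automatic editor regeneration with a billboard indicator.
; Destruction also removes directly attached actors; the vegetation update is an empty stub.
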(event EventDestroyed
  (CallFunction|Destroy))

(fn ConstructionScript
  (CallFunction|Generate))

(fn Destroy
  (for _array_element (Actor|GetAttachedActors true false)
    (Utilities|Array|AddUnique (LocalVariables|GetAllActors) _array_element))
  (for _array_element_2 (LocalVariables|GetAllActors)
    (Actor|DestroyActor _array_element_2))
  (Actor|DestroyActor))

(fn Generate
  (bind (_origin _boxextent) (Collision|GetActorBounds false true))
  (Class|PCGComponent|SetGraph (Variables|Default|GetPCG) (Variables|Data|GetPCG%20Graph))
  (bind _fence (Variables|Props|GetFence)
    (:then
      (CallFunction|UpdateVillageFences _fence)
      (LocalVariables|SetOrigin _origin)
      (Transformation|SetWorldLocation (Variables|Default|GetCube) _origin false false)
      (Transformation|SetWorldScale3D (Variables|Default|GetCube) _boxextent)
      (Transformation|SetWorldLocation (Variables|Default|GetBillboard) (Math|Vector|MakeVector (.x (LocalVariables|GetOrigin)) (.y (LocalVariables|GetOrigin)) (+ (.z (LocalVariables|GetOrigin)) 1e+03)) false false))
    (:else)))

(fn UpdateVegetation
  (params (ST_VegetationDensity :type ST%20Vegetation%20Density%20Structure%20%28by%20ref%29)))

(fn UpdateSmallFences
  (params (InputPin :type PDA%20Village%20Object%20Object%20Reference))
  (bind _structout (Utilities|Struct|SetmembersinST_Object (Utilities|Array|Get(acopy) (Variables|/Game/Massive/MassiveVillage/Data/Structure/PDA_VillageObject.PDA_VillageObject_C|GetMeshes InputPin))))
  (Variables|Data|SetSmall%20Fence%20Length (Math|Float|Clamp(Float) (* (.x (.boxextent (StaticMesh|GetBounds (.mesh _structout)))) 2.0) 25.0 1e+03))
  (return))

(fn ForceUpdate
  (bind _spline (Variables|Default|GetSpline))
  (Spline|SetLocationatSplinePoint _spline 0 (+ (.position (Spline|GetSplinePointAt _spline 0 "Local")) "0.100000,0.000000,0.100000") "Local" true)
  (Spline|UpdateSpline _spline)
  (Class|PCGComponent|GenerateLocal (Variables|Default|GetPCG) true))

(fn UpdateVillageFences
  (params (InputPin :type PDA%20Village%20Object%20Object%20Reference))
  (bind _structout (Utilities|Struct|SetmembersinST_Object (Utilities|Array|Get(acopy) (Variables|/Game/Massive/MassiveVillage/Data/Structure/PDA_VillageObject.PDA_VillageObject_C|GetMeshes InputPin))))
  (Variables|Data|SetVillage%20Fence%20Length (Math|Float|Clamp(Float) (* (.x (.boxextent (StaticMesh|GetBounds (.mesh _structout)))) 2.0) 25.0 1e+03))
  (return))

(fn Clear
  (Class|PCGComponent|Cleanup (Variables|Default|GetPCG) true false))

(fn ToggleAutoPCGUpdate
  (if (Variables|Data|GetUpdateLandscape?)
    ;[0.02522 0.249 0.07835] Auto Update PCG
    (Variables|Data|SetUpdateLandscape? false)
    (Variables|/Script/PCG.PCGComponent|SetbRegenerateInEditor (Variables|Default|GetPCG) true)
    (Rendering|SetVisibility (Variables|Default|GetBillboardUpdate) true false)
    (PCG|Generate (Variables|Default|GetPCG) true)
    (else
      ;[1 0.2691 0.2433] Stop Auto Update PCG
      (Variables|Data|SetUpdateLandscape? true)
      (Variables|/Script/PCG.PCGComponent|SetbRegenerateInEditor (Variables|Default|GetPCG) false)
      (Rendering|SetVisibility (Variables|Default|GetBillboardUpdate) false false)
      (PCG|Generate (Variables|Default|GetPCG) true))))