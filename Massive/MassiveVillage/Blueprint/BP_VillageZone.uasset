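; BP_VillageZone is a spline-based zone marker for the village, typed as Residential, Marketplace or one of several numbered regions.
; On construction it replaces its actor tags with the zone type's name, so the type is readable as a tag.
; It also picks a billboard sprite matching the type and places it above the averaged position of the spline points.
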(fn ConstructionScript
  (Utilities|Array|Clear (Variables|Actor|GetTags))
  (Utilities|Array|AddUnique (Variables|Actor|GetTags) (Utilities|String|StringToName (Utilities|String|EnumtoString (Variables|Default|GetZone%20Type))))
  (CallFunction|ForceUpdate)
  (CallFunction|GetCenterPosition))

(fn ForceUpdate
  (Utilities|Array|Clear (Variables|Actor|GetTags))
  (Utilities|Array|AddUnique (Variables|Actor|GetTags) (Utilities|String|StringToName (Utilities|String|EnumtoString (Variables|Default|GetZone%20Type))))
  (Rendering|Components|Sprite|SetSprite (Variables|Default|GetBillboard) (Utilities|Select :Index (Variables|Default|GetZone%20Type) :NewEnumerator0 "/Game/Massive/MassiveVillage/Texture/UI/Resident.Resident" :NewEnumerator1 "/Game/Massive/MassiveVillage/Texture/UI/Market.Market" :NewEnumerator2 "/Game/Massive/MassiveVillage/Texture/UI/Three.Three" :NewEnumerator3 "/Game/Massive/MassiveVillage/Texture/UI/Four.Four" :NewEnumerator4 "/Game/Massive/MassiveVillage/Texture/UI/Five.Five")))

(fn GetCenterPosition
  (bind _spline (Variables|Default|GetSpline))
  (bind _returnvalue (Spline|GetNumberOfSplinePoints _spline))
  (LocalVariables|SetPositionSum "0, 0, 0")
  (Utilities|Array|Clear (LocalVariables|GetPosition))
  (LocalVariables|SetNumber%20of%20Points _returnvalue)
  (for _index (range 1 _returnvalue)
    (Utilities|Array|AddUnique (LocalVariables|GetPosition) (.position (Spline|GetSplinePointAt (Variables|Default|GetSpline) _index "Local"))))
  (for _array_element (LocalVariables|GetPosition)
    (LocalVariables|SetPositionSum (+ (LocalVariables|GetPositionSum) _array_element)))
  (Transformation|SetRelativeLocation (Variables|Default|GetBillboard) (+ (/ (LocalVariables|GetPositionSum) (LocalVariables|GetNumber%20of%20Points)) "0.000000,0.000000,1000.000000") false false))