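; BP_DragMaster is an editor Blueprint whose one function shown, GetActorToIgnore, rebuilds a list of actors to exclude; the file does not show what uses it.
; It clears ActorsToIgnore, then adds every actor carrying a TagToIgnore tag and every PCGPartitionActor, without duplicates.
; The child-actor pass runs after the partition loop, so it adds descendants of only the last partition actor.
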(fn GetActortoIgnore
  (Utilities|Array|Clear (Variables|Default|GetActors%20to%20Ignore))
  (for _array_element (Variables|Default|GetTagToIgnore)
    (bind _outactors (Actor|GetAllActorswithTag _array_element))
    (for _array_element_2 _outactors
      (Utilities|Array|AddUnique (Variables|Default|GetActors%20to%20Ignore) _array_element_2)))
  (bind _outactors_2 (Actor|GetAllActorsOfClass "/Script/PCG.PCGPartitionActor"))
  (for _array_element_3 _outactors_2
    (Utilities|Array|AddUnique (Variables|Default|GetActors%20to%20Ignore) _array_element_3))
  (for _array_element_4 (Actor|GetAllChildActors _array_element_3 true)
    (Utilities|Array|AddUnique (Variables|Default|GetActors%20to%20Ignore) _array_element_4))
  (return))