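; Editor scriptable tool for debugging line traces, showing what lies under the cursor during a drag.
; Drag updates fire a long Visibility trace along the cursor's world ray and cache the hit result.
; The HUD draws location, actor, component, physical material, distance and hit state at that point, recolored red on a miss.
; A BP_DebugProperty settings set is restored on setup and saved on shutdown, but the trace and drawing never read it.
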(event EventOnScriptSetup
  (bind _returnvalue (Class|ScriptableInteractiveTool|AddPropertySetOfType "/Game/Massive/MassiveShared/Blueprint/Editor/BP_DebugProperty.BP_DebugProperty_C" "DebugSettings")
    (:Success
      (bind _output_get (Variables|Default|SetProperty _returnvalue))
      (Class|ScriptableInteractiveTool|RestorePropertySetSettings _output_get "DebugSettings"))))

(event EventOnScriptShutdown
  (params (ShutdownType :type EToolShutdownType%20Enum :default "Completed"))
  (Class|ScriptableInteractiveTool|SavePropertySetSettings (Variables|Default|GetProperty) "DebugSettings"))

(event EventOnScriptDrawHUD
  (params (DrawHUDAPI :type Scriptable%20Tool%20HUDAPI%20Object%20Reference))
  (bind _return_hit (Variables|Default|GetReturn%20Hit))
  (bind _out_hit_hit_actor (Variables|Default|GetOut%20Hit%20Hit%20Actor))
  (bind _draw_location (Variables|Default|GetDraw%20Location))
  (bind _out_hit_phys_mat (Variables|Default|GetOut%20Hit%20Phys%20Mat))
  (bind _out_hit_distance (Variables|Default|GetOut%20Hit%20Distance))
  (bind _out_hit_hit_component (Variables|Default|GetOut%20Hit%20Hit%20Component))
  (bind _returnvalue (Utilities|String|ToString(Vector) _draw_location))
  (bind _returnvalue_2 (Utilities|GetDisplayName _out_hit_phys_mat))
  (bind _returnvalue_3 (Utilities|String|ToString(Float) _out_hit_distance))
  (bind _returnvalue_4 (Utilities|GetDisplayName _out_hit_hit_component))
  (bind _returnvalue_5 (Utilities|String|ToString(Boolean) _return_hit))
  (bind _returnvalue_6 (Utilities|GetDisplayName _out_hit_hit_actor))
  (bind _returnvalue_7 (Utilities|String|Append "Return hit = " _returnvalue_5))
  (bind _returnvalue_8 (Utilities|String|Append "Location =  " _returnvalue))
  (bind _returnvalue_9 (Utilities|String|Append "Hit Actor = " _returnvalue_6))
  (bind _returnvalue_10 (Utilities|String|Append "Hit Component = " _returnvalue_4))
  (bind _returnvalue_11 (Utilities|String|Append "Physical Material = " _returnvalue_2))
  (bind _returnvalue_12 (Utilities|String|Append "Hit Distance = " _returnvalue_3))
  (bind _array (Utilities|Array|MakeArray _returnvalue_8 _returnvalue_9 _returnvalue_10 _returnvalue_11 _returnvalue_12 _returnvalue_7))
  (if (Variables|Default|GetReturn%20Hit)
    (Class|ScriptableToolHUDAPI|DrawTextArrayatLocation DrawHUDAPI (Variables|Default|GetDraw%20Location) _array "(R=1.0,G=1.0,B=1.0,A=1.0)" false 2.0)
    (else
      (Class|ScriptableToolHUDAPI|DrawTextArrayatLocation DrawHUDAPI (Variables|Default|GetDraw%20Location) _array "(R=0.682292,G=0.000000,B=0.017765,A=1.000000)" false 2.0))))

(event EventOnDragUpdatePosition
  (params (NewPosition :type Input%20Device%20Ray%20Structure) (Modifiers :type Scriptable%20Tool%20Modifier%20States%20Structure%20%28by%20ref%29))
  (bind _worldray (Utilities|Struct|BreakInputDeviceRay NewPosition))
  (bind _worldray_2 (Utilities|Struct|BreakInputDeviceRay (Utilities|Struct|MakeInputDeviceRay _worldray false "(X=0.000000,Y=0.000000)")))
  (bind (_outhit _returnvalue) (Collision|LineTraceByChannel (.origin _worldray_2) (+ (.origin _worldray_2) (* (.direction _worldray_2) 5e+06)) "TraceTypeQuery1" false 0 "ForOneFrame" true "(R=1.000000,G=0.000000,B=0.403293,A=1.000000)"))
  (Variables|Default|SetDraw%20Location (.location _outhit))
  (Variables|Default|SetOut%20Hit%20Hit%20Actor (.hitactor _outhit))
  (Variables|Default|SetOut%20Hit%20Phys%20Mat (.physmat _outhit))
  (Variables|Default|SetOut%20Hit%20Distance (.distance _outhit))
  (Variables|Default|SetOut%20Hit%20Hit%20Component (.hitcomponent _outhit))
  (Variables|Default|SetReturn%20Hit _returnvalue))

(fn OnHoverUpdate
  (params (HoverPos :type Input%20Device%20Ray%20Structure) (Modifiers :type Scriptable%20Tool%20Modifier%20States%20Structure%20%28by%20ref%29))
  (return false))