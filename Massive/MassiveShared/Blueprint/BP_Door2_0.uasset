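; Door actor that swings open or closed each time its Open/CloseDoor event is called.
; A FlipFlop alternates between playing and reversing a timeline, whose float drives a yaw lerp on the static mesh's relative rotation.
; UpdateDoorMesh applies the Door mesh variable, or prints a message if it is invalid; nothing in this file calls it.
; The construction script only calls its parent.
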(event Custom|Open%20/%20Close%20Door
  (Utilities|FlowControl|FlipFlop
    (:A
      (bind _doortimerfloat (Timeline|Timeline_0 PlayFromStart)
        (:Update
          (Transformation|SetRelativeRotation (Variables|Default|GetStaticMesh) (Math|Rotator|MakeRotator 0.0 0.0 (Math|Float|Lerp 0.0 8e+01 _doortimerfloat)) false false))))
    (:B
      (Timeline|Timeline_0 ReverseFromEnd))))

(fn ConstructionScript
  (|CallParentFunction))

(fn UpdateDoorMesh
  (bind _door (Variables|Default|GetDoor)
    (:then
      (Components|StaticMesh|SetStaticMesh (Variables|Default|GetStaticMesh) _door))
    (:else
      (Development|PrintString "Could not find any doors"))))