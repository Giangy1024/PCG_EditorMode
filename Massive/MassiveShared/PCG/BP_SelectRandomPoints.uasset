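; Custom PCG Blueprint element, shown as "Select Random Point", that marks a random PointsToSelect-sized subset of each spatial input's points.
; It shuffles point indices with the context's seeded random stream and takes the first entries.
; Selected points get Density 1 and the rest 0, so none are removed, and tags and pins carry through.
; The clamp for counts exceeding the available points is unconnected, and index arrays are not cleared between inputs.
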(fn ExecutewithContext
  (params (InContext :type PCG%20Context%20Structure%20%28by%20ref%29) (Input :type PCG%20Data%20Collection%20Structure%20%28by%20ref%29))
  (bind _returnvalue (Class|PCGDataFunctionLibrary|GetInputs Input))
  (for _array_element _returnvalue
    (LocalVariables|SetTags (.Tags (Utilities|Struct|BreakPCGTaggedData _array_element)))
    (LocalVariables|SetPin (.Pin (Utilities|Struct|BreakPCGTaggedData _array_element)))
    (bind _aspcgspatial_data (Utilities|Casting|CastToPCGSpatialData (.Data (Utilities|Struct|BreakPCGTaggedData _array_element))))
    (bind _output_get (LocalVariables|SetPointData (SpatialData|ToPointDatawithContext _aspcgspatial_data InContext)))
    (bind _output_get_2 (LocalVariables|SetAllPoints (SpatialData|GetPoints _output_get)))
    (LocalVariables|SetCounts (Utilities|Array|Length _output_get_2))
    (LocalVariables|SetSelectedMax (> (Variables|Default|GetPoints%20to%20select) (LocalVariables|GetCounts)))
    (for _index (range 0 (LocalVariables|GetCounts))
      (Utilities|Array|Add (LocalVariables|GetAllIndex) _index))
    (bind _returnvalue_2 (Class|PCGBlueprintElement|GetRandomStream InContext))
    (Utilities|Array|ShuffleFromStream (LocalVariables|GetAllIndex) _returnvalue_2)
    (if (LocalVariables|GetSelectedMax)
      _
      (else
        _))
    (for _index_2 (range 0 (- (Variables|Default|GetPoints%20to%20select) 1))
      (Utilities|Array|Add (LocalVariables|GetIndexToSelect) (Utilities|Array|Get(acopy) (LocalVariables|GetAllIndex) _index_2)))
    (for (_array_element_2 _array_index) (LocalVariables|GetAllPoints)
      (bind _structout (Utilities|Struct|SetmembersinPCGPoint _array_element_2 0.0))
      (Utilities|Array|SetArrayElem (LocalVariables|GetAllPoints) _array_index _structout))
    (for (_array_element_3 _array_index_2) (LocalVariables|GetAllPoints)
      (for _array_element_4 (LocalVariables|GetIndexToSelect)
        (if (== _array_element_4 _array_index_2)
          (bind _structout_2 (Utilities|Struct|SetmembersinPCGPoint _array_element_3 1.0))
          (Utilities|Array|SetArrayElem (LocalVariables|GetAllPoints) _array_index_2 _structout_2))))
    (SpatialData|SetPoints (LocalVariables|GetPointData) (LocalVariables|GetAllPoints))
    (Utilities|Array|Add (LocalVariables|GetOutTaggedData) (Utilities|Struct|MakePCGTaggedData (LocalVariables|GetPointData) (LocalVariables|GetTags) (LocalVariables|GetPin))))
  (return (Utilities|Struct|MakePCGDataCollection (LocalVariables|GetOutTaggedData))))

(fn NodeTitleOverride
  (return "Select Random Point"))